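; BP_GameManager tracks player insanity and the lighting state for the spooky VR factory game.
; Init starts two looping one-second timers: one raises insanity up to a cap, the other counts down until the lights fail.
; Lights going out increases the insanity multiplier, while EnableLights reverses that and randomizes the next countdown.
; TakePill lowers insanity, and each sanity or light change fires an event dispatcher.
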(event `self.ReceiveInit`
  (`KismetSystemLibrary.K2_SetTimerDelegate` (delegate `StartSanityDrop`) 1.0 true)
  (`KismetSystemLibrary.K2_SetTimerDelegate` (delegate `Lights`) 1.0 true))

(event `StartSanityDrop`
  (set `self.Insanity` (`KismetMathLibrary.FMin` 100.0 (+ (`self.Insanity`) (* (`self.PassiveSanityDrop`) (`self.InsanityMultiplier`)))))
  (`self.SanityDropped`))

(event `Lights`
  (if (`self.AreLightsOn`)
    (bind _result (`/Engine/EditorBlueprintResources/StandardMacros.DecrementFloat` (`self.LightTimer`))
      (:`  `
        (if (<= _result 0.0)
          (`self.LightsOff`)
          (set `self.AreLightsOn` false)
          (`/Engine/EditorBlueprintResources/StandardMacros.IncrementFloat` (`self.InsanityMultiplier`)))))))

(fn `EnableLights`
  (`self.LightsOn`)
  (set `self.AreLightsOn` true)
  (`/Engine/EditorBlueprintResources/StandardMacros.DecrementFloat` (`self.InsanityMultiplier`)
    (:`  `
      (set `self.LightTimer` (+ (`self.MinLightOnTime`) (* (`KismetMathLibrary.RandomFloat`) (- (`self.MaxLightOnTime`) (`self.MinLightOnTime`))))))))

(fn `Take Pill`
  (bind _insanity (`self.Insanity`))
  (set `self.Insanity` (- _insanity (`KismetMathLibrary.FMin` _insanity (`self.PillRestorationAmount`))))
  (`self.SanityRestored`))