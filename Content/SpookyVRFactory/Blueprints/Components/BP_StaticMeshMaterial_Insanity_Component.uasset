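; Component that swaps a named material slot on a static mesh according to the player's insanity level.
; On BeginPlay it binds one check to the BP_GameManager game instance's sanity dropped and restored events.
; The check lazily caches sorted float threshold keys from a material map, applies the material for the first one Insanity meets or exceeds, then fires an object-changed dispatcher.
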(event `self.ReceiveBeginPlay`
  (bind _asbp_game_manager (cast `/Game/SpookyVRFactory/Blueprints/BP_GameManager` (`GameplayStatics.GetGameInstance`)))
  (bind _output_get (set `self.Game Manager` _asbp_game_manager))
  (add `/Game/SpookyVRFactory/Blueprints/BP_GameManager.SanityDropped` _output_get (delegate `CheckSanity`))
  (add `/Game/SpookyVRFactory/Blueprints/BP_GameManager.SanityRestored` _output_get (delegate `CheckSanity`)))

(event `CheckSanity`
  (if (`KismetArrayLibrary.Array_IsEmpty` (`self.InsanityLevels`))
    (bind _keys (`BlueprintMapLibrary.Map_Keys` (`self.Materials`)))
    (bind _output_get (set `self.InsanityLevels` _keys))
    (`KismetArrayLibrary.SortFloatArray` _output_get false "Descending"))
  (for _array_element (`self.InsanityLevels`)
    (if (>= (`/Game/SpookyVRFactory/Blueprints/BP_GameManager.Insanity` (`self.Game Manager`)) _array_element)
      (`PrimitiveComponent.SetMaterialByName` (`self.StaticMeshComponent`) (`self.MaterialName`) (`BlueprintMapLibrary.Map_Find` (`self.Materials`) _array_element))
      (`self.ObjectChanged`)
      (break))))