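; BP_Dog is a dog that grows hungry over time and turns hangry when hunger and the game's Insanity are both high.
; A looping timer raises HungerLevel up to MaxHunger, while Feed lowers it.
; Both re-evaluate Hangry against the chase threshold and the GameManager game instance's Insanity.
; The attack is a placeholder: Tick prints a debug message while Hangry, and the stored player reference is unused.
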(event `self.ReceiveBeginPlay`
  (`KismetSystemLibrary.K2_SetTimerDelegate` (delegate `Hungerer`) 5.0 true)
  (set `self.Player` (`GameplayStatics.GetPlayerCharacter` 0))
  (bind _asbp_game_manager (cast `/Game/SpookyVRFactory/Blueprints/BP_GameManager` (`GameplayStatics.GetGameInstance`)))
  (set `self.GameManager` _asbp_game_manager))

(event `Hungerer`
  (bind _result (`/Engine/EditorBlueprintResources/StandardMacros.IncrementInt` (`self.HungerLevel`))
    (:`  `
      (if (> _result (`self.MaxHunger`))
        (set `self.HungerLevel` (`self.MaxHunger`)))
      (`self.CheckHungerLevel`))))

(event `Feed`
  (set `self.HungerLevel` (- (`self.HungerLevel`) 5))
  (`self.CheckHungerLevel`))

(event `CheckHungerLevel`
  (set `self.Hangry` (and (>= (`self.HungerLevel`) (`self.HungerLimitToChase`)) (>= (`/Game/SpookyVRFactory/Blueprints/BP_GameManager.Insanity` (`self.GameManager`)) 75.0))))

(event `self.ReceiveTick`
  (params (DeltaSeconds :type "Float (single-precision)"))
  (if (`self.Hangry`)
    (`KismetSystemLibrary.PrintString` "Dog Attack")))

(fn `UserConstructionScript`)