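; Grabbable VR robot torso that players assemble by attaching buildable parts to head, legs and arm sockets.
; Range overlaps highlight indicators and arm an attach, which Tick completes by snapping the part once released; indicators show open sockets while the base is held.
; Socket maps track occupancy and correctness, with build status printed only after correct placements.
; Part detach callbacks reset their socket, and Destoy destroys all attached actors.
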(event `self.ReceiveTick`
  (params (DeltaSeconds :type "Float (single-precision)"))
  (bind _as_bp_buildable_object_part (`self.As BP Buildable Object Part`))
  ;[0.07118 0.0336 0.06229] Attach the part to the socket once the player lets go of the object
  (if (`self.TryAttach`)
    (if (not (`/Game/SpookyVRFactory/Blueprints/Objects/BP_Buildable_Object_Part.Grabbing` _as_bp_buildable_object_part))
      (`self.K2_AttachToActor` _as_bp_buildable_object_part self (`KismetStringLibrary.Conv_StringToName` (`self.CurrentAttachmentPoint`)) "SnapToTarget" "SnapToTarget" "KeepWorld" true)
      (set `self.TryAttach` false)
      (set `/Game/SpookyVRFactory/Blueprints/Objects/BP_Buildable_Object_Part.Attached` true _as_bp_buildable_object_part)
      (`PrimitiveComponent.SetSimulatePhysics` (`/Game/SpookyVRFactory/Blueprints/Objects/BP_Buildable_Object_Part.StaticMesh` _as_bp_buildable_object_part) false)
      (`BlueprintMapLibrary.Map_Add` (`self.IsAttached`) (`self.CurrentAttachmentPoint`) true)
      (`self.ShowAttachmentPoint` false)
      ;[0.08607 0.2066 0.05756] Check if the robot is correctly built
      (if (== (`/Game/SpookyVRFactory/Blueprints/Objects/BP_Buildable_Object_Part.CorrectSocket` (`self.As BP Buildable Object Part`)) (`self.CurrentAttachmentPoint`))
        (`BlueprintMapLibrary.Map_Add` (`self.Correct`) (`self.CurrentAttachmentPoint`) true)
        (bind _values (`BlueprintMapLibrary.Map_Values` (`self.Correct`)))
        (for _array_element _values
          (if _array_element
            (set `self.FullyBuilt` true)
            (else
              (set `self.FullyBuilt` false)
              (break))))
        (bind _values_2 (`BlueprintMapLibrary.Map_Values` (`self.IsAttached`)))
        (for _array_element_2 _values_2
          (if _array_element_2
            (set `self.hasPart` true)
            (else
              (set `self.hasPart` false)
              (break))))
        (if (`self.hasPart`)
          (if (`self.FullyBuilt`)
            (`KismetSystemLibrary.PrintString` "Correct" true true (struct :`R` 0.086069 :`G` 0.206597 :`B` 0.057559 :`A` 1.0) 102.0)
            (else
              (`KismetSystemLibrary.PrintString` "WrongParts" true true (struct :`R` 0.092014 :`G` 0.047233 :`B` 0.012143 :`A` 1.0) 102.0)))
          (else
            (`KismetSystemLibrary.PrintString` "NotBuilt" true true (struct :`R` 0.07118 :`G` 0.033602 :`B` 0.062286 :`A` 1.0) 102.0)))))))

(event `self.ReceiveBeginPlay`)

(event `self.GrabComponent.OnGrabbed`
  (set `self.Holding` true)
  (`self.ShowAttachmentPoint` false))

(event `self.GrabComponent.OnDropped`
  (set `self.Holding` false)
  (`self.ShowAttachmentPoint` true))

(event `self.HeadHighlightRange.OnComponentBeginOverlap`
  (params (OverlappedComponent :type "PrimitiveComponent Object Reference") (OtherActor :type "Actor Object Reference") (OtherComp :type "PrimitiveComponent Object Reference") (OtherBodyIndex :type Integer) (bFromSweep :type Boolean) (SweepResult :type "HitResult Structure (by ref)"))
  (bind (_value _returnvalue) (`BlueprintMapLibrary.Map_Find` (`self.IsAttached`) (`KismetSystemLibrary.GetObjectName` (`self.Head`))))
  ;[0.07118 0.0336 0.06229] Prepare to attach a part to the head socket
  (bind _asbp_buildable_object_part (cast `/Game/SpookyVRFactory/Blueprints/Objects/BP_Buildable_Object_Part` OtherActor))
  (if _returnvalue
    (if (not _value)
      (`PrimitiveComponent.SetMaterial` (`self.HeadIndicator`) 0 "/DatasmithContent/Materials/AliasReference.AliasReference" :!label _label)
      (if (`/Game/SpookyVRFactory/Blueprints/Objects/BP_Buildable_Object_Part.Grabbing` _asbp_buildable_object_part)
        (set `self.TryAttach` true)
        (set `self.CurrentAttachmentPoint` "Socket_Head")
        (bind _output_get (set `self.As BP Buildable Object Part` _asbp_buildable_object_part))
        (add `/Game/SpookyVRFactory/Blueprints/Objects/BP_Buildable_Object_Part.Detach` _output_get (delegate `DetachHead`))))
    (else
      (goto _label))))

(event `DetachHead`
  ;[0.09201 0.04723 0.01214] Select which socket to show after detach
  (`self.Detach` (`self.HeadIndicator`) "Socket_Head"))

(event `self.HeadHighlightRange.OnComponentEndOverlap`
  (params (OverlappedComponent :type "PrimitiveComponent Object Reference") (OtherActor :type "Actor Object Reference") (OtherComp :type "PrimitiveComponent Object Reference") (OtherBodyIndex :type Integer))
  ;[0.08854 0.08217 0.04057] Cancel the attachment to the head socket
  (cast `/Game/SpookyVRFactory/Blueprints/Objects/BP_Buildable_Object_Part` OtherActor)
  (`PrimitiveComponent.SetMaterial` (`self.HeadIndicator`) 0 "/Engine/BasicShapes/BasicShapeMaterial.BasicShapeMaterial")
  (set `self.TryAttach` false))

(event `self.LegsHighlightRange.OnComponentBeginOverlap`
  (params (OverlappedComponent :type "PrimitiveComponent Object Reference") (OtherActor :type "Actor Object Reference") (OtherComp :type "PrimitiveComponent Object Reference") (OtherBodyIndex :type Integer) (bFromSweep :type Boolean) (SweepResult :type "HitResult Structure (by ref)"))
  (bind (_value _returnvalue) (`BlueprintMapLibrary.Map_Find` (`self.IsAttached`) (`KismetSystemLibrary.GetObjectName` (`self.Legs`))))
  ;[0.07118 0.0336 0.06229] Prepare to attach a part to the leg socket
  (bind _asbp_buildable_object_part (cast `/Game/SpookyVRFactory/Blueprints/Objects/BP_Buildable_Object_Part` OtherActor))
  (if _returnvalue
    (if (not _value)
      (`PrimitiveComponent.SetMaterial` (`self.LegsIndicator`) 0 "/DatasmithContent/Materials/AliasReference.AliasReference" :!label _label_2)
      (if (`/Game/SpookyVRFactory/Blueprints/Objects/BP_Buildable_Object_Part.Grabbing` _asbp_buildable_object_part)
        (set `self.TryAttach` true)
        (set `self.CurrentAttachmentPoint` "Socket_Legs")
        (bind _output_get (set `self.As BP Buildable Object Part` _asbp_buildable_object_part))
        (add `/Game/SpookyVRFactory/Blueprints/Objects/BP_Buildable_Object_Part.Detach` _output_get (delegate `DeatchLeg`))))
    (else
      (goto _label_2))))

(event `DeatchLeg`
  ;[0.09201 0.04723 0.01214] Select which slot to show after detach
  (`self.Detach` (`self.LegsIndicator`) "Socket_Legs"))

(event `self.LegsHighlightRange.OnComponentEndOverlap`
  (params (OverlappedComponent :type "PrimitiveComponent Object Reference") (OtherActor :type "Actor Object Reference") (OtherComp :type "PrimitiveComponent Object Reference") (OtherBodyIndex :type Integer))
  ;[0.08854 0.08217 0.04057] Cancle the attachment to the leg socket
  (cast `/Game/SpookyVRFactory/Blueprints/Objects/BP_Buildable_Object_Part` OtherActor)
  (`PrimitiveComponent.SetMaterial` (`self.LegsIndicator`) 0 "/Engine/BasicShapes/BasicShapeMaterial.BasicShapeMaterial")
  (set `self.TryAttach` false))

(event `Detach`
  (params (HighlightPoint :type "PrimitiveComponent Object Reference") (AttachmentPoint :type String))
  ;[0.09201 0.04723 0.01214] Remove the attached object and show the attachment point again
  (`PrimitiveComponent.SetMaterial` HighlightPoint 0 "/Engine/BasicShapes/BasicShapeMaterial.BasicShapeMaterial")
  (set `self.TryAttach` false)
  (`BlueprintMapLibrary.Map_Add` (`self.IsAttached`) AttachmentPoint)
  (`self.ShowAttachmentPoint` false)
  (`BlueprintMapLibrary.Map_Add` (`self.Correct`) AttachmentPoint))

(event `self.LeftArmHilightRange.OnComponentBeginOverlap`
  (params (OverlappedComponent :type "PrimitiveComponent Object Reference") (OtherActor :type "Actor Object Reference") (OtherComp :type "PrimitiveComponent Object Reference") (OtherBodyIndex :type Integer) (bFromSweep :type Boolean) (SweepResult :type "HitResult Structure (by ref)"))
  (bind (_value _returnvalue) (`BlueprintMapLibrary.Map_Find` (`self.IsAttached`) (`KismetSystemLibrary.GetObjectName` (`self.LeftArm`))))
  ;[0.07118 0.0336 0.06229] Prepare to attach a part to the LeftArm socket
  (bind _asbp_buildable_object_part (cast `/Game/SpookyVRFactory/Blueprints/Objects/BP_Buildable_Object_Part` OtherActor))
  (if _returnvalue
    (if (not _value)
      (`PrimitiveComponent.SetMaterial` (`self.LeftArmIndicator`) 0 "/DatasmithContent/Materials/AliasReference.AliasReference" :!label _label_3)
      (if (`/Game/SpookyVRFactory/Blueprints/Objects/BP_Buildable_Object_Part.Grabbing` _asbp_buildable_object_part)
        (set `self.TryAttach` true)
        (set `self.CurrentAttachmentPoint` "Socket_Arm_Left")
        (bind _output_get (set `self.As BP Buildable Object Part` _asbp_buildable_object_part))
        (add `/Game/SpookyVRFactory/Blueprints/Objects/BP_Buildable_Object_Part.Detach` _output_get (delegate `DetachLeftArm`))))
    (else
      (goto _label_3))))

(event `DetachLeftArm`
  ;[0.09201 0.04723 0.01214] Select which socket to show after detach
  (`self.Detach` (`self.LeftArmIndicator`) "Socket_Arm_Left"))

(event `self.LeftArmHilightRange.OnComponentEndOverlap`
  (params (OverlappedComponent :type "PrimitiveComponent Object Reference") (OtherActor :type "Actor Object Reference") (OtherComp :type "PrimitiveComponent Object Reference") (OtherBodyIndex :type Integer))
  ;[0.08854 0.08217 0.04057] Cancle the attachment to the LeftArm socket
  (cast `/Game/SpookyVRFactory/Blueprints/Objects/BP_Buildable_Object_Part` OtherActor)
  (`PrimitiveComponent.SetMaterial` (`self.LeftArmIndicator`) 0 "/Engine/BasicShapes/BasicShapeMaterial.BasicShapeMaterial")
  (set `self.TryAttach` false))

(event `self.RightArmHighlightRange.OnComponentBeginOverlap`
  (params (OverlappedComponent :type "PrimitiveComponent Object Reference") (OtherActor :type "Actor Object Reference") (OtherComp :type "PrimitiveComponent Object Reference") (OtherBodyIndex :type Integer) (bFromSweep :type Boolean) (SweepResult :type "HitResult Structure (by ref)"))
  (bind (_value _returnvalue) (`BlueprintMapLibrary.Map_Find` (`self.IsAttached`) (`KismetSystemLibrary.GetObjectName` (`self.RightArm`))))
  ;[0.07118 0.0336 0.06229] Prepare to attach a part to the LeftArm socket
  (bind _asbp_buildable_object_part (cast `/Game/SpookyVRFactory/Blueprints/Objects/BP_Buildable_Object_Part` OtherActor))
  (if _returnvalue
    (if (not _value)
      (`PrimitiveComponent.SetMaterial` (`self.RightArmIndicator`) 0 "/DatasmithContent/Materials/AliasReference.AliasReference" :!label _label_4)
      (if (`/Game/SpookyVRFactory/Blueprints/Objects/BP_Buildable_Object_Part.Grabbing` _asbp_buildable_object_part)
        (set `self.TryAttach` true)
        (set `self.CurrentAttachmentPoint` "Socket_Arm_Right")
        (bind _output_get (set `self.As BP Buildable Object Part` _asbp_buildable_object_part))
        (add `/Game/SpookyVRFactory/Blueprints/Objects/BP_Buildable_Object_Part.Detach` _output_get (delegate `DetachRightArm`))))
    (else
      (goto _label_4))))

(event `DetachRightArm`
  ;[0.09201 0.04723 0.01214] Select which socket to show after detach
  (`self.Detach` (`self.RightArmIndicator`) "Socket_Arm_Right"))

(event `self.RightArmHighlightRange.OnComponentEndOverlap`
  (params (OverlappedComponent :type "PrimitiveComponent Object Reference") (OtherActor :type "Actor Object Reference") (OtherComp :type "PrimitiveComponent Object Reference") (OtherBodyIndex :type Integer))
  ;[0.08854 0.08217 0.04057] Cancle the attachment to the RightArm socket
  (cast `/Game/SpookyVRFactory/Blueprints/Objects/BP_Buildable_Object_Part` OtherActor)
  (`PrimitiveComponent.SetMaterial` (`self.RightArmIndicator`) 0 "/Engine/BasicShapes/BasicShapeMaterial.BasicShapeMaterial")
  (set `self.TryAttach` false))

(fn `Destoy`
  (set `self.destroying` true)
  (for _array_element (`self.GetAttachedActors` true true)
    (`self.K2_DestroyActor` _array_element)))

(fn `ShowAttachmentPoint`
  (params (VisibilityOverride :type Boolean))
  (if (`self.Holding`)
    (if VisibilityOverride
      (`SceneComponent.SetVisibility` (`self.HeadIndicator`) false false :!label _label)
      (`SceneComponent.SetVisibility` (`self.LegsIndicator`) false false)
      (`SceneComponent.SetVisibility` (`self.LeftArmIndicator`) false false)
      (`SceneComponent.SetVisibility` (`self.RightArmIndicator`) false false)
      (else
        (`SceneComponent.SetVisibility` (`self.HeadIndicator`) (not (`BlueprintMapLibrary.Map_Find` (`self.IsAttached`) (`KismetStringLibrary.Concat_StrStr` "Socket_" (`KismetSystemLibrary.GetObjectName` (`self.Head`))))) false)
        (`SceneComponent.SetVisibility` (`self.LegsIndicator`) (not (`BlueprintMapLibrary.Map_Find` (`self.IsAttached`) (`KismetStringLibrary.Concat_StrStr` "Socket_" (`KismetSystemLibrary.GetObjectName` (`self.Legs`))))) false)
        (`SceneComponent.SetVisibility` (`self.LeftArmIndicator`) (not (`BlueprintMapLibrary.Map_Find` (`self.IsAttached`) "Socket_Arm_Left")) false)
        (`SceneComponent.SetVisibility` (`self.RightArmIndicator`) (not (`BlueprintMapLibrary.Map_Find` (`self.IsAttached`) "Socket_Arm_Right")) false)))
    (else
      (goto _label))))

(fn `UserConstructionScript`)