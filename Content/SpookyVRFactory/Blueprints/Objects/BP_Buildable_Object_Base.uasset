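; Base Blueprint for a grabbable buildable object in the VR factory, with Arm and Leg sockets that accept BP_Buildable_Object_Part actors.
; Overlapping a socket's range highlights its sphere and arms attachment for held parts; Tick snaps the part on once released, disabling its physics.
; An IsAttached map tracks filled sockets, and per-socket detach callbacks clear them.
; Free socket markers show on grab; ShowAttachmentPoint's true input hides all markers.
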(event `self.ReceiveTick`
  (params (DeltaSeconds :type "Float (single-precision)"))
  (bind _as_bp_buildable_object_part (`self.As BP Buildable Object Part`))
  ;[0.07118 0.0336 0.06229] Attach the part to the socket once the player lets go of the object
  (if (`self.TryAttach`)
    (if (not (`/Game/SpookyVRFactory/Blueprints/Objects/BP_Buildable_Object_Part.Grabbing` _as_bp_buildable_object_part))
      (`self.K2_AttachToComponent` _as_bp_buildable_object_part (`self.CurrentAttachmentPoint`) "None" "SnapToTarget" "SnapToTarget" "KeepWorld" true)
      (set `self.TryAttach` false)
      (set `/Game/SpookyVRFactory/Blueprints/Objects/BP_Buildable_Object_Part.Attached` true _as_bp_buildable_object_part)
      (`PrimitiveComponent.SetSimulatePhysics` (`/Game/SpookyVRFactory/Blueprints/Objects/BP_Buildable_Object_Part.StaticMesh` _as_bp_buildable_object_part) false)
      (`BlueprintMapLibrary.Map_Add` (`self.IsAttached`) (`KismetSystemLibrary.GetObjectName` (`self.CurrentAttachmentPoint`)) true)
      (`self.ShowAttachmentPoint` false))))

(event `self.GrabComponent.OnGrabbed`
  (`self.ShowAttachmentPoint` false))

(event `self.GrabComponent.OnDropped`
  (`self.ShowAttachmentPoint` true))

(event `self.HighlightRange.OnComponentBeginOverlap`
  (params (OverlappedComponent :type "PrimitiveComponent Object Reference") (OtherActor :type "Actor Object Reference") (OtherComp :type "PrimitiveComponent Object Reference") (OtherBodyIndex :type Integer) (bFromSweep :type Boolean) (SweepResult :type "HitResult Structure (by ref)"))
  ;[0.07118 0.0336 0.06229] Prepare to attach a part to the arm socket
  (bind _asbp_buildable_object_part (cast `/Game/SpookyVRFactory/Blueprints/Objects/BP_Buildable_Object_Part` OtherActor))
  (`PrimitiveComponent.SetMaterial` (`self.Sphere`) 0 "/DatasmithContent/Materials/AliasReference.AliasReference")
  (if (`/Game/SpookyVRFactory/Blueprints/Objects/BP_Buildable_Object_Part.Grabbing` _asbp_buildable_object_part)
    (set `self.TryAttach` true)
    (set `self.CurrentAttachmentPoint` (`self.Arm`))
    (bind _output_get (set `self.As BP Buildable Object Part` _asbp_buildable_object_part))
    (add `/Game/SpookyVRFactory/Blueprints/Objects/BP_Buildable_Object_Part.Detach` _output_get (delegate `DetachArm`))))

(event `DetachArm`
  ;[0.09201 0.04723 0.01214] Select which socket to show after detach
  (`self.Detach` (`self.Sphere`) (`KismetSystemLibrary.GetObjectName` (`self.Arm`))))

(event `self.HighlightRange.OnComponentEndOverlap`
  (params (OverlappedComponent :type "PrimitiveComponent Object Reference") (OtherActor :type "Actor Object Reference") (OtherComp :type "PrimitiveComponent Object Reference") (OtherBodyIndex :type Integer))
  ;[0.08854 0.08217 0.04057] Cancel the attachment to the arm socket
  (cast `/Game/SpookyVRFactory/Blueprints/Objects/BP_Buildable_Object_Part` OtherActor)
  (`PrimitiveComponent.SetMaterial` (`self.Sphere`) 0 "/Engine/BasicShapes/BasicShapeMaterial.BasicShapeMaterial")
  (set `self.TryAttach` false))

(event `Detach`
  (params (HighlightPoint :type "PrimitiveComponent Object Reference") (AttachmentPoint :type String))
  ;[0.09201 0.04723 0.01214] Remove the attached object and show the attachment point again
  (`PrimitiveComponent.SetMaterial` HighlightPoint 0 "/Engine/BasicShapes/BasicShapeMaterial.BasicShapeMaterial")
  (set `self.TryAttach` false)
  (`BlueprintMapLibrary.Map_Add` (`self.IsAttached`) AttachmentPoint)
  (`self.ShowAttachmentPoint` false))

(event `self.HighlightRange1.OnComponentBeginOverlap`
  (params (OverlappedComponent :type "PrimitiveComponent Object Reference") (OtherActor :type "Actor Object Reference") (OtherComp :type "PrimitiveComponent Object Reference") (OtherBodyIndex :type Integer) (bFromSweep :type Boolean) (SweepResult :type "HitResult Structure (by ref)"))
  ;[0.07118 0.0336 0.06229] Prepare to attach a part to the leg socket
  (bind _asbp_buildable_object_part (cast `/Game/SpookyVRFactory/Blueprints/Objects/BP_Buildable_Object_Part` OtherActor))
  (`PrimitiveComponent.SetMaterial` (`self.Sphere1`) 0 "/DatasmithContent/Materials/AliasReference.AliasReference")
  (if (`/Game/SpookyVRFactory/Blueprints/Objects/BP_Buildable_Object_Part.Grabbing` _asbp_buildable_object_part)
    (set `self.TryAttach` true)
    (set `self.CurrentAttachmentPoint` (`self.Leg`))
    (bind _output_get (set `self.As BP Buildable Object Part` _asbp_buildable_object_part))
    (add `/Game/SpookyVRFactory/Blueprints/Objects/BP_Buildable_Object_Part.Detach` _output_get (delegate `DeatchLeg`))))

(event `DeatchLeg`
  ;[0.09201 0.04723 0.01214] Select which slot to show after detach
  (`self.Detach` (`self.Sphere1`) (`KismetSystemLibrary.GetObjectName` (`self.Leg`))))

(event `self.HighlightRange1.OnComponentEndOverlap`
  (params (OverlappedComponent :type "PrimitiveComponent Object Reference") (OtherActor :type "Actor Object Reference") (OtherComp :type "PrimitiveComponent Object Reference") (OtherBodyIndex :type Integer))
  ;[0.08854 0.08217 0.04057] Cancle the attachment to the leg socket
  (cast `/Game/SpookyVRFactory/Blueprints/Objects/BP_Buildable_Object_Part` OtherActor)
  (`PrimitiveComponent.SetMaterial` (`self.Sphere1`) 0 "/Engine/BasicShapes/BasicShapeMaterial.BasicShapeMaterial")
  (set `self.TryAttach` false))

(fn `ShowAttachmentPoint`
  (params (VisibilityOverride :type Boolean))
  (if VisibilityOverride
    (`SceneComponent.SetVisibility` (`self.Sphere`) false false)
    (`SceneComponent.SetVisibility` (`self.Sphere1`) false false)
    (else
      (`SceneComponent.SetVisibility` (`self.Sphere`) (not (`BlueprintMapLibrary.Map_Find` (`self.IsAttached`) (`KismetSystemLibrary.GetObjectName` (`self.Arm`)))) false)
      (`SceneComponent.SetVisibility` (`self.Sphere1`) (not (`BlueprintMapLibrary.Map_Find` (`self.IsAttached`) (`KismetSystemLibrary.GetObjectName` (`self.Leg`)))) false))))

(fn `UserConstructionScript`)