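; BP_Buildable_Object_Part is a grabbable part of a buildable object, tracking whether it is held and whether it is attached.
; Grabbing it through GrabComponent sets the Grabbing state and, if the part is attached, clears Attached and calls CallDetach.
; Dropping it clears Grabbing and turns on physics simulation for the mesh.
; An unconnected branch that would toggle mesh collision by attachment state never runs.
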(event `self.ReceiveTick`
  (params (DeltaSeconds :type "Float (single-precision)")))

(event `self.GrabComponent.OnGrabbed`
  (set `self.Grabbing` true)
  (if (`self.Attached`)
    (set `self.Attached` false)
    (`self.Detach`)))

(event `self.GrabComponent.OnDropped`
  (set `self.Grabbing` false)
  (`PrimitiveComponent.SetSimulatePhysics` (`self.StaticMesh`) true))

(fn `UserConstructionScript`)