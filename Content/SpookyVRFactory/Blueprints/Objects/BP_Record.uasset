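; BP_Record is a grabbable vinyl record that spins on a turntable while music plays in the VR factory.
; A looping timer rotates the static mesh in small steps from BeginPlay.
; Grabbing clears the timer, stops the audio, plays a record-stop sound and, after a delay, a boss voice line reacting to the music.
; Dropping it turns on physics simulation for the mesh.
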(event `self.ReceiveBeginPlay`
  (bind _returnvalue (`KismetSystemLibrary.K2_SetTimerDelegate` (delegate `Event_Rotate`) 0.05 true)))

(event `Event_Rotate`
  (`SceneComponent.K2_AddRelativeRotation` (`self.StaticMesh`) (struct :`Yaw` 20.0) false false))

(event `self.GrabComponent.OnGrabbed`
  (`KismetSystemLibrary.K2_ClearAndInvalidateTimerHandle` (stale `self.ReceiveBeginPlay` _returnvalue))
  (`AudioComponent.Stop` (`self.Audio`))
  (`GameplayStatics.PlaySound2D` "/Game/SpookyVRFactory/Audio/Effects/Turntable_Record_Stop_01.Turntable_Record_Stop_01" 1.0 1.0 0.0 null null)
  (`KismetSystemLibrary.Delay` 2.0)
  (`GameplayStatics.PlaySound2D` "/Game/SpookyVRFactory/Audio/Effects/Boss_DontLikeMusic.Boss_DontLikeMusic" 2.5 1.0 0.0 null null))

(event `self.GrabComponent.OnDropped`
  (`PrimitiveComponent.SetSimulatePhysics` (`self.StaticMesh`) true))

(fn `UserConstructionScript`)