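; Quota board that shows the current quota as a two-digit seven-segment display on a static mesh.
; On BeginPlay it reads the quota from BP_GameManager (the game instance) and binds to its quota-change event to refresh.
; The value splits into tens and units, and each digit maps to segments lit by swapping named material slots, with Left-/Right- prefixes, between red light and cable materials.
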(event `self.ReceiveBeginPlay`
  (bind _asbp_game_manager (cast `/Game/SpookyVRFactory/Blueprints/BP_GameManager` (`GameplayStatics.GetGameInstance`)))
  (set `self.As BP Game Manager` _asbp_game_manager)
  (`self.Display Quota` (`/Game/SpookyVRFactory/Blueprints/BP_GameManager.Quota` _asbp_game_manager))
  (add `/Game/SpookyVRFactory/Blueprints/BP_GameManager.QuotaChange` _asbp_game_manager (delegate `Quota`)))

(event `Quota`
  (`self.Display Quota` (`/Game/SpookyVRFactory/Blueprints/BP_GameManager.Quota` (`self.As BP Game Manager`))))

(fn `Display Quota`
  (params (Quota :type Integer))
  (locals (FirstNumber :type Integer :default 0) (SecondNumber :type Integer :default 0))
  (bind _output_get (set `local.FirstNumber` (`KismetMathLibrary.FTrunc` (/ (`KismetMathLibrary.Conv_IntToDouble` Quota) 10.0))))
  (bind _output_get_2 (set `local.SecondNumber` (mod Quota 10)))
  (`self.DisplayNumber` _output_get true)
  (`self.DisplayNumber` _output_get_2))

(fn `DisplayNumber`
  (params (Number :type Integer) (FirstNumber :type Boolean))
  (locals (Prefix :type Name :default "None"))
  (bind _prefix (`local.Prefix`))
  (if FirstNumber
    (set `local.Prefix` "Left-")
    (else
      (set `local.Prefix` "Right-")))
  (switch `int` Number
    (:`0`
      (`self.SetMaterials` _prefix true true false true true true true))
    (:`1`
      (`self.SetMaterials` _prefix false false false true false false true))
    (:`2`
      (`self.SetMaterials` _prefix true true true false false true true))
    (:`3`
      (`self.SetMaterials` _prefix true false true true false true true))
    (:`4`
      (`self.SetMaterials` _prefix false false true true true false true))
    (:`5`
      (`self.SetMaterials` _prefix true false true true true true))
    (:`6`
      (`self.SetMaterials` _prefix true true true true true true))
    (:`7`
      (`self.SetMaterials` _prefix false false false true false true true))
    (:`8`
      (`self.SetMaterials` _prefix true true true true true true true))
    (:`9`
      (`self.SetMaterials` _prefix false false true true true true true))))

(fn `SetMaterials`
  (params (Prefix :type Name) (Bottom :type Boolean) (BottomLeft :type Boolean) (Middle :type Boolean) (BottomRight :type Boolean) (TopLeft :type Boolean) (Top :type Boolean) (TopRight :type Boolean))
  (bind _returnvalue (`KismetStringLibrary.Conv_NameToString` Prefix))
  (bind _staticmesh (`self.StaticMesh`))
  (bind _staticmesh_2 (`self.StaticMesh`))
  (bind _staticmesh_3 (`self.StaticMesh`))
  (bind _staticmesh_4 (`self.StaticMesh`))
  (bind _staticmesh_5 (`self.StaticMesh`))
  (bind _staticmesh_6 (`self.StaticMesh`))
  (bind _staticmesh_7 (`self.StaticMesh`))
  (bind _returnvalue_2 (`KismetStringLibrary.Concat_StrStr` _returnvalue "Up-Right"))
  (bind _returnvalue_3 (`KismetStringLibrary.Concat_StrStr` _returnvalue "Bottom"))
  (bind _returnvalue_4 (`KismetStringLibrary.Concat_StrStr` _returnvalue "Bottom-Left"))
  (bind _returnvalue_5 (`KismetStringLibrary.Concat_StrStr` _returnvalue "Middle"))
  (bind _returnvalue_6 (`KismetStringLibrary.Concat_StrStr` _returnvalue "Bottom-Right"))
  (bind _returnvalue_7 (`KismetStringLibrary.Concat_StrStr` _returnvalue "Up-Left"))
  (bind _returnvalue_8 (`KismetStringLibrary.Concat_StrStr` _returnvalue "Up"))
  (if Bottom
    (`PrimitiveComponent.SetMaterialByName` _staticmesh_2 (`KismetStringLibrary.Conv_StringToName` _returnvalue_3) "/Game/SpookyVRFactory/Materials/M_RedLight.M_RedLight")
    (else
      (`PrimitiveComponent.SetMaterialByName` _staticmesh_2 (`KismetStringLibrary.Conv_StringToName` _returnvalue_3) "/Game/SpookyVRFactory/Materials/M_Cable.M_Cable")))
  (if BottomLeft
    (`PrimitiveComponent.SetMaterialByName` _staticmesh_3 (`KismetStringLibrary.Conv_StringToName` _returnvalue_4) "/Game/SpookyVRFactory/Materials/M_RedLight.M_RedLight")
    (else
      (`PrimitiveComponent.SetMaterialByName` _staticmesh_3 (`KismetStringLibrary.Conv_StringToName` _returnvalue_4) "/Game/SpookyVRFactory/Materials/M_Cable.M_Cable")))
  (if Middle
    (`PrimitiveComponent.SetMaterialByName` _staticmesh_4 (`KismetStringLibrary.Conv_StringToName` _returnvalue_5) "/Game/SpookyVRFactory/Materials/M_RedLight.M_RedLight")
    (else
      (`PrimitiveComponent.SetMaterialByName` _staticmesh_4 (`KismetStringLibrary.Conv_StringToName` _returnvalue_5) "/Game/SpookyVRFactory/Materials/M_Cable.M_Cable")))
  (if BottomRight
    (`PrimitiveComponent.SetMaterialByName` _staticmesh_5 (`KismetStringLibrary.Conv_StringToName` _returnvalue_6) "/Game/SpookyVRFactory/Materials/M_RedLight.M_RedLight")
    (else
      (`PrimitiveComponent.SetMaterialByName` _staticmesh_5 (`KismetStringLibrary.Conv_StringToName` _returnvalue_6) "/Game/SpookyVRFactory/Materials/M_Cable.M_Cable")))
  (if TopLeft
    (`PrimitiveComponent.SetMaterialByName` _staticmesh_6 (`KismetStringLibrary.Conv_StringToName` _returnvalue_7) "/Game/SpookyVRFactory/Materials/M_RedLight.M_RedLight")
    (else
      (`PrimitiveComponent.SetMaterialByName` _staticmesh_6 (`KismetStringLibrary.Conv_StringToName` _returnvalue_7) "/Game/SpookyVRFactory/Materials/M_Cable.M_Cable")))
  (if Top
    (`PrimitiveComponent.SetMaterialByName` _staticmesh_7 (`KismetStringLibrary.Conv_StringToName` _returnvalue_8) "/Game/SpookyVRFactory/Materials/M_RedLight.M_RedLight")
    (else
      (`PrimitiveComponent.SetMaterialByName` _staticmesh_7 (`KismetStringLibrary.Conv_StringToName` _returnvalue_8) "/Game/SpookyVRFactory/Materials/M_Cable.M_Cable")))
  (if TopRight
    (`PrimitiveComponent.SetMaterialByName` _staticmesh (`KismetStringLibrary.Conv_StringToName` _returnvalue_2) "/Game/SpookyVRFactory/Materials/M_RedLight.M_RedLight")
    (else
      (`PrimitiveComponent.SetMaterialByName` _staticmesh (`KismetStringLibrary.Conv_StringToName` _returnvalue_2) "/Game/SpookyVRFactory/Materials/M_Cable.M_Cable"))))

(fn `UserConstructionScript`)