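; BP_LightObject is a light fixture in SpookyVRFactory that switches on and off with the game's global lighting events.
; On BeginPlay it casts the game instance to BP_GameManager and binds its On and Off events to the manager's lights-on and lights-off events.
; Each event shows or hides the Meshes component with its children and swaps the Bulb material between emissive-style M_Light and plain glass.
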(event `self.ReceiveBeginPlay`
  (bind _asbp_game_manager (cast `/Game/SpookyVRFactory/Blueprints/BP_GameManager` (`GameplayStatics.GetGameInstance`)))
  (add `/Game/SpookyVRFactory/Blueprints/BP_GameManager.LightsOn` _asbp_game_manager (delegate `On`))
  (add `/Game/SpookyVRFactory/Blueprints/BP_GameManager.LightsOff` _asbp_game_manager (delegate `Off`)))

(event `On`
  (`SceneComponent.SetVisibility` (`self.meshes`) true true)
  (`PrimitiveComponent.SetMaterial` (`self.bulb`) 0 "/Game/SpookyVRFactory/Materials/M_Light.M_Light"))

(event `Off`
  (`SceneComponent.SetVisibility` (`self.meshes`) false true)
  (`PrimitiveComponent.SetMaterial` (`self.bulb`) 0 "/Game/AdvancedGlassPack/Materials/01_Clean/M_Glass_CleanMaster.M_Glass_CleanMaster"))

(fn `UserConstructionScript`)