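; BP_Button_Machine is a pressable button that powers on the machine in SpookyVRFactory.
; When the VR pawn overlaps its box, the button slides down, plays a power-on sound and calls EventPowerOn on the BP_Machine found by class lookup.
; It then slides back to its start position, with a Moving flag blocking re-triggers during the motion.
; A game-manager lights check is present but unconnected.
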(event `self.ReceiveBeginPlay`
  (set `self.ButtonStart` (`SceneComponent.RelativeLocation` (`self.Button`))))

(event `self.Box.OnComponentBeginOverlap`
  (params (OverlappedComponent :type "PrimitiveComponent Object Reference") (OtherActor :type "Actor Object Reference") (OtherComp :type "PrimitiveComponent Object Reference") (OtherBodyIndex :type Integer) (bFromSweep :type Boolean) (SweepResult :type "HitResult Structure (by ref)"))
  (if (not (`self.Moving`))
    (cast `/Game/VRTemplate/Blueprints/VRPawn` OtherActor)
    (set `self.Moving` true)
    (`KismetSystemLibrary.MoveComponentTo` (`self.Button`) (- (`self.ButtonStart`) (0.0 0.0 5.0)))
    (`GameplayStatics.PlaySoundAtLocation` "/Game/SpookyVRFactory/Audio/Effects/Retro_Radio_Power_On_04.Retro_Radio_Power_On_04" (`self.K2_GetActorLocation`) (struct) 1.0 1.0 0.0 null null null null)
    (bind _returnvalue (`GameplayStatics.GetActorOfClass` "/Game/SpookyVRFactory/Blueprints/BP_Machine.BP_Machine_C"))
    (`/Game/SpookyVRFactory/Blueprints/BP_Machine.Event_PowerOn` _returnvalue)
    (`self.Return`)))

(event `Return`
  (`KismetSystemLibrary.MoveComponentTo` (`self.Button`) (`self.ButtonStart`))
  (set `self.Moving` false))

(fn `UserConstructionScript`)