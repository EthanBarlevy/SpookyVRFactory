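; BP_MenuButton is a configurable menu button in SpookyVRFactory, built from a cube and a text label.
; Its Click event switches on ButtonType to either open the level named by LevelName or quit the game.
; Highlight and unhighlight events swap the cube between HighlightMaterial and BaseMaterial, and the construction script applies the display text and base material.
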(event `Click`
  (switch `/Game/SpookyVRFactory/Enums/E_ButtonType` (`self.ButtonType`)
    (:`NewEnumerator0`
      (`GameplayStatics.OpenLevel` (`KismetStringLibrary.Conv_StringToName` (`self.LevelName`))))
    (:`NewEnumerator1`
      (`KismetSystemLibrary.QuitGame` null "Quit"))))

(event `HighlightButton`
  (`PrimitiveComponent.SetMaterial` (`self.Cube`) 0 (`self.HighlightMaterial`)))

(event `UnhighlightButton`
  (`PrimitiveComponent.SetMaterial` (`self.Cube`) 0 (`self.BaseMaterial`)))

(fn `UserConstructionScript`
  (`TextRenderComponent.K2_SetText` (`self.TextRender`) (`KismetTextLibrary.Conv_StringToText` (`self.DisplayText`)))
  (`PrimitiveComponent.SetMaterial` (`self.Cube`) 0 (`self.BaseMaterial`)))