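; BP_Lever is a VR grabbable lever that turns the lights back on through BP_GameManager.
; When the grab component is dropped with the mesh near its on rotation, within a tolerance, it calls the game manager's lights-on.
; It binds to the manager's lights-off event at BeginPlay and snaps the mesh to the opposite rotation when that fires.
; It also gathers all BP_LightObject actors, but never uses them here.
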(event `self.ReceiveBeginPlay`
  (bind _outactors (`GameplayStatics.GetAllActorsOfClass` "/Game/SpookyVRFactory/Blueprints/Objects/BP_LightObject.BP_LightObject_C"))
  (set `self.Lights` _outactors)
  (bind _asbp_game_manager (cast `/Game/SpookyVRFactory/Blueprints/BP_GameManager` (`GameplayStatics.GetGameInstance`)))
  (add `/Game/SpookyVRFactory/Blueprints/BP_GameManager.LightsOff` _asbp_game_manager (delegate `Event_OnLightsOff`)))

(event `Event_OnLightsOff`
  (`SceneComponent.K2_SetRelativeRotation` (`self.StaticMesh`) (struct :`Roll` 90.0) false false))

(event `self.GrabComponent.OnDropped`
  (if (== (`SceneComponent.RelativeRotation` (`self.StaticMesh`)) (struct :`Roll` -90.0) :`ErrorTolerance` 20.0)
    (bind _asbp_game_manager (cast `/Game/SpookyVRFactory/Blueprints/BP_GameManager` (`GameplayStatics.GetGameInstance`)))
    (`/Game/SpookyVRFactory/Blueprints/BP_GameManager.LightsOn` _asbp_game_manager)))

(fn `UserConstructionScript`)