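; Factory machine that spawns BP_Robot actors in response to sanity drops and has two counter-rotating cogs.
; Binds to BP_GameManager's sanity events; each drop starts a delay, then spawns a robot at a random point within its Box bounds.
; SpawnTime shortens that delay in steps as Insanity rises, while the sanity-restored handler is empty.
; A fast looping timer, rather than Tick, appears to drive the cog rotation.
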(event `self.ReceiveBeginPlay`
  (bind _asbp_game_manager (cast `/Game/SpookyVRFactory/Blueprints/BP_GameManager` (`GameplayStatics.GetGameInstance`)))
  (bind _output_get (set `self.BP_GameManager` _asbp_game_manager))
  (add `/Game/SpookyVRFactory/Blueprints/BP_GameManager.SanityDropped` _output_get (delegate `Event_SanityDroped`))
  (add `/Game/SpookyVRFactory/Blueprints/BP_GameManager.SanityRestored` (`self.BP_GameManager`) (delegate `Event_SanityRestored`))
  (`KismetSystemLibrary.K2_SetTimerDelegate` (`|CreateDelegate` :!event `Event_RotateCogs`) 0.005 true))

(event `Event_SanityDroped`
  (bind (_origin _boxextent) (`KismetSystemLibrary.GetComponentBounds` (`self.Box`)))
  (bind _spawnrate (`self.SpawnTime`))
  (`KismetSystemLibrary.Delay` _spawnrate)
  (`|SpawnActorFromClass` "/Game/SpookyVRFactory/Blueprints/BP_Robot.BP_Robot_C" (`KismetMathLibrary.MakeTransform` (`KismetMathLibrary.RandomPointInBoundingBox` _origin _boxextent)) "Undefined" "MultiplyWithRoot" null null))

(event `Event_SanityRestored`)

(event `Event_RotateCogs`
  (`SceneComponent.K2_AddLocalRotation` (`self.OtherCog`) (struct :`Yaw` 0.5) false false)
  (`SceneComponent.K2_AddLocalRotation` (`self.Cog`) (struct :`Yaw` -0.5) false false))

(fn `SpawnTime`
  (returns (SpawnRate :type "Float (double-precision)"))
  (if (`KismetMathLibrary.InRange_FloatFloat` (`/Game/SpookyVRFactory/Blueprints/BP_GameManager.Insanity` (`self.BP_GameManager`)) 0.0 20.0 true false)
    (return 5.0)
    (elif (`KismetMathLibrary.InRange_FloatFloat` (`/Game/SpookyVRFactory/Blueprints/BP_GameManager.Insanity` (`self.BP_GameManager`)) 20.0 40.0 true false)
      (return 4.0)
      (elif (`KismetMathLibrary.InRange_FloatFloat` (`/Game/SpookyVRFactory/Blueprints/BP_GameManager.Insanity` (`self.BP_GameManager`)) 40.0 60.0 true false)
        (return 3.0)
        (elif (`KismetMathLibrary.InRange_FloatFloat` (`/Game/SpookyVRFactory/Blueprints/BP_GameManager.Insanity` (`self.BP_GameManager`)) 60.0 80.0 true false)
          (return 2.0)
          (elif (`KismetMathLibrary.InRange_FloatFloat` (`/Game/SpookyVRFactory/Blueprints/BP_GameManager.Insanity` (`self.BP_GameManager`)) 80.0 100.0)
            (return 1.0)))))))

(fn `UserConstructionScript`)