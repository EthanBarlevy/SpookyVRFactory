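; Base Blueprint for breakable props that shatter on a hard impact, pairing an intact static mesh with a Geometry Collection.
; A mesh hit with velocity above ImpactTolerance calls Break, which detaches the collection in place, enables its physics, crumbles the cluster, plays a sound and destroys the intact mesh.
; Five seconds later, physics simulation on the debris is switched off.
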(event `self.ReceiveBeginPlay`)

(event `self.StaticMesh.OnComponentHit`
  (params (HitComponent :type "PrimitiveComponent Object Reference") (OtherActor :type "Actor Object Reference") (OtherComp :type "PrimitiveComponent Object Reference") (NormalImpulse :type "Vector Structure") (Hit :type "HitResult Structure (by ref)"))
  (if (> (`KismetMathLibrary.VSize` (`SceneComponent.GetComponentVelocity` (`self.StaticMesh`))) (`self.ImpactTolerance`))
    (`self.Break`)
    (`KismetSystemLibrary.Delay` 5.0)
    (`PrimitiveComponent.SetSimulatePhysics` (`self.GeometryCollection`) false)))

(fn `Break`
  (bind _geometrycollection (`self.GeometryCollection`))
  (`SceneComponent.K2_DetachFromComponent` (`self.GeometryCollection`) "KeepWorld" "KeepWorld" "KeepWorld" true)
  (`PrimitiveComponent.SetSimulatePhysics` (`self.GeometryCollection`) true)
  (`GeometryCollectionComponent.CrumbleCluster` _geometrycollection 0)
  (`GameplayStatics.PlaySoundAtLocation` (`self.BreakSound`) (`SceneComponent.K2_GetComponentLocation` _geometrycollection) (struct) 1.0 1.0 0.0 null null null null)
  (`ActorComponent.K2_DestroyComponent` (`self.StaticMesh`)))

(fn `UserConstructionScript`)